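; Building Blueprint that procedurally assembles a block structure from static mesh components in its Construction Script; the event graph is unused.
; Nested Z, Y and X loops fill the whole volume on a 100-unit grid, sized by XNum, YNum and ZNum.
; The ground-level front-row cell at Entranceint gets an entrance mesh picked from EnterMesh by MeshNum; every other cell uses NewMesh.
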(fn `UserConstructionScript`
  ;[1 1 1] z축 반복
  (for _index (range (+ (`self.Z Num`) 1))
    ;[1 1 1] y축 반복
    (for _index_2 (range (+ (`self.Y Num`) 1))
      ;[1 1 1] x축 반복
      (for _index_3 (range (+ (`self.X Num`) 1))
        ;[1 1 1] meshOption
        (bind _returnvalue (`AddComponent|NODE_AddStaticMeshComponent-0` :`RelativeTransform` (`KismetMathLibrary.MakeTransform` (`KismetMathLibrary.MakeVector` (* _index_3 100.0) (* _index_2 100.0) (* _index 100.0)))))
        (if (== _index 0)
          (if (== _index_2 0)
            (if (== _index_3 (`self.entranceint`))
              (`StaticMeshComponent.SetStaticMesh` _returnvalue (`|GetArrayItem` (`self.enter Mesh`) (`self.meshNum`)))
              (else
                (`StaticMeshComponent.SetStaticMesh` _returnvalue (`self.New Mesh`) :!label _label)
                (`PrimitiveComponent.SetMaterial` _returnvalue 0 null)))
            (else
              (goto _label)))
          (else
            (goto _label)))))))